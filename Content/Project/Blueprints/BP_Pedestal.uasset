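; BP_Pedestal is a pedestal actor that accepts a key and shows a decorative key once one is placed.
; Its box overlap detects BP_Key entering or leaving and, unless already placed, tells BP_Manager whether that key can go on this pedestal.
; The PlaceToPedestal event toggles the decorative key's visibility, while BP_Manager, found at BeginPlay, receives the overlap notices.
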(event OnComponentBeginOverlap(Box)
  (params (OverlappedComponent :type Primitive%20Component%20Object%20Reference) (OtherActor :type Actor%20Object%20Reference) (OtherComp :type Primitive%20Component%20Object%20Reference) (OtherBodyIndex :type Integer) (bFromSweep :type Boolean) (SweepResult :type Hit%20Result%20Structure%20%28by%20ref%29))
  (Utilities|Casting|CastToBP_Key OtherActor)
  (if (not (stale Custom|PlaceToPedestal Placed))
    (Default|KeytoPedestal (Variables|Default|GetBP_Manager) self true)))

(event OnComponentEndOverlap(Box)
  (params (OverlappedComponent :type Primitive%20Component%20Object%20Reference) (OtherActor :type Actor%20Object%20Reference) (OtherComp :type Primitive%20Component%20Object%20Reference) (OtherBodyIndex :type Integer))
  (Utilities|Casting|CastToBP_Key OtherActor)
  (if (not (stale Custom|PlaceToPedestal Placed))
    (Default|KeytoPedestal (Variables|Default|GetBP_Manager) 0 false)))

(event Custom|PlaceToPedestal
  (params (Placed :type Boolean))
  (Rendering|SetVisibility (Variables|Default|GetBP_KeyDecorative) Placed false))

(event EventBeginPlay
  (bind _returnvalue (Actor|GetActorOfClass "/Game/Project/Blueprints/BP_Manager.BP_Manager_C"))
  (Variables|Default|SetBP_Manager _returnvalue))

(fn ConstructionScript)