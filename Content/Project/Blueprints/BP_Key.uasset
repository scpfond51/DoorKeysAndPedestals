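; BP_Key is a key actor with a Collect event that receives and stores the first-person player.
; A FlipFlop makes every second Collect call start a looping timer that runs MoveKey.
; MoveKey applies a zero rotation and offsets the key by its own world location, doubling its position each tick of the timer.
; The motion looks unfinished, as the lookup of the player's PlaceForKey location is left unconnected.
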(event Custom|Collect
  (params (BP_FirstPerson :type BP%20First%20Person%20Character%20Object%20Reference))
  (Variables|Default|SetBP_FirstPerson BP_FirstPerson)
  (Utilities|FlowControl|FlipFlop
    (:B
      (Utilities|Time|SetTimerbyEvent (delegate Custom|MoveKey) 0.1 true))))

(event Custom|MoveKey
  (Class|Actor|AddActorWorldRotation "0, 0, 0")
  (Transformation|AddActorWorldOffset (* (Transformation|GetActorLocation) "1.000000,1.000000,1.000000")))

(fn ConstructionScript)