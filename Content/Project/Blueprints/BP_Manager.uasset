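; BP_Manager is a manager Blueprint that handles key pickup through a line trace from the first-person camera.
; On BeginPlay it finds and caches the BP_FirstPersonCharacter.
; Its LineTraceClick event runs a Visibility trace along the camera's forward vector, with debug drawing left on.
; If the hit actor is a BP_Key, it calls Collect on the key and passes in the character.
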(event Custom|GetActors
  ;[0.15 0.15 0.15 0.5] GetActors
  (bind _returnvalue (Actor|GetActorOfClass "/Game/FirstPerson/Blueprints/BP_FirstPersonCharacter.BP_FirstPersonCharacter_C"))
  (Variables|Default|SetBP_FirstPerson _returnvalue))

(event Custom|LineTraceClick
  ;[0.15 0.15 0.15 0.5] LineTrace
  (bind _out_hit (CallFunction|LineTraceSystem (Variables|Default|GetLine%20Trace%20Range)))
  (bind _asbp_key (Utilities|Casting|CastToBP_Key (.HitActor (Collision|BreakHitResult _out_hit))))
  (Default|Collect _asbp_key (Variables|Default|GetBP_FirstPerson)))

(event EventBeginPlay
  ;[0.15 0.15 0.15 0.5] Event BeginPlay
  (CallFunction|GetActors))

(fn ConstructionScript)

(fn LineTraceSystem
  (params (LineTraceRange :type Vector))
  (bind _bp_firstperson (Variables|Default|GetBP_FirstPerson))
  (bind _firstpersoncamera (Variables|/Game/FirstPerson/Blueprints/BP_FirstPersonCharacter.BP_FirstPersonCharacter_C|GetFirstPersonCamera _bp_firstperson))
  (bind _returnvalue (Transformation|GetWorldLocation _firstpersoncamera))
  ;[0.15 0.15 0.15 0.5] LineTrace
  (bind _outhit (Collision|LineTraceByChannel _returnvalue (+ _returnvalue (* (Math|Vector|GetForwardVector (Transformation|GetWorldRotation (Variables|/Game/FirstPerson/Blueprints/BP_FirstPersonCharacter.BP_FirstPersonCharacter_C|GetFirstPersonCamera (Variables|Default|GetBP_FirstPerson)))) LineTraceRange)) "TraceTypeQuery1" false 0 "ForDuration" true "(R=1.000000,G=0.000000,B=0.000000,A=1.000000)" "(R=0.000000,G=1.000000,B=0.000000,A=1.000000)" 1.0))
  (return _outhit))