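; BP_Door is a puzzle door that swings its mesh to a fixed rotation once every pedestal sharing its ID is placed.
; On BeginPlay it finds BP_Manager and binds to its door-update event.
; Each update scans all BP_Pedestal actors, counting matching IDs and how many are placed.
; It requires at least one matching pedestal and never rotates back.
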(event Custom|GetActors
  ;[0.15 0.15 0.15 0.5] GetActors
  (bind _returnvalue (Actor|GetActorOfClass "/Game/Project/Blueprints/BP_Manager.BP_Manager_C"))
  (Variables|Default|SetBP_Manager _returnvalue))

(event Custom|EventUpdateDoor
  ;[0.15 0.15 0.15 0.5] UpdateDoor
  (EventDispatchers|BindEventtoUpdateDoor (Variables|Default|GetBP_Manager) (delegate Custom|UpdateDoor)))

(event Custom|UpdateDoor
  ;[0.15 0.15 0.15 0.5] UpdateDoor
  (Variables|Default|SetCountOfPedestals 0)
  (Variables|Default|SetEndedPedestals 0)
  (bind _outactors (Actor|GetAllActorsOfClass "/Game/Project/Blueprints/BP_Pedestal.BP_Pedestal_C"))
  (for _array_element _outactors
    (if (== (Variables|/Game/Project/Blueprints/BP_Pedestal.BP_Pedestal_C|GetID _array_element) (Variables|Default|GetID))
      (Variables|Default|SetCountOfPedestals (+ (Variables|Default|GetCountOfPedestals) 1))
      (if (Variables|/Game/Project/Blueprints/BP_Pedestal.BP_Pedestal_C|GetPlaced _array_element)
        (Variables|Default|SetEndedPedestals (+ (Variables|Default|GetEndedPedestals) 1)))))
  (if (and (> (Variables|Default|GetCountOfPedestals) 0) (== (Variables|Default|GetCountOfPedestals) (Variables|Default|GetEndedPedestals)))
    (Transformation|SetWorldRotation (Variables|Default|GetStaticMesh) "0.000000,90.000000,0.000000" false false)))

(event EventBeginPlay
  ;[0.15 0.15 0.15 0.5] EventBeginPlay
  (CallFunction|GetActors)
  (CallFunction|EventUpdateDoor))

(fn ConstructionScript)